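; BP_Player is the player pawn with Enhanced Input movement, look, jump and boost, using the IMC_Sonic mapping.
; Moving turns the actor to the spring arm's yaw and roll.
; Boost raises max walk speed and loops forward-vector impulses, scaled only on world X, with no delay.
; While boosting, Tick drives a dynamic blur-vignette post-process material from horizontal velocity; releasing boost restores run speed and clears the blur.
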(event Input|EnhancedActionEvents|EnhancedInputActionIA_Move
  (params (ActionValue :type Vector%202D%20Structure) (ElapsedSeconds :type Float%20%28double-precision%29) (TriggeredSeconds :type Float%20%28double-precision%29) (InputAction :type Input%20Action%20Object%20Reference :default "/Game/Blueprints/Player/Input/IA_Move.IA_Move"))
  (bind _springarm (Variables|Default|GetSpringArm))
  (bind _returnvalue (Class|SpringArmComponent|GetTargetRotation _springarm))
  (Pawn|Input|AddMovementInput (Transformation|GetActorForwardVector) (.x ActionValue) false)
  (Pawn|Input|AddMovementInput (Transformation|GetActorRightVector) (.y ActionValue) false)
  (Transformation|SetActorRotation (Math|Rotator|MakeRotator (.roll _returnvalue) 0.0 (.yaw _returnvalue))))

(event Input|EnhancedActionEvents|EnhancedInputActionIA_Look
  (params (ActionValue :type Vector%202D%20Structure) (ElapsedSeconds :type Float%20%28double-precision%29) (TriggeredSeconds :type Float%20%28double-precision%29) (InputAction :type Input%20Action%20Object%20Reference :default "/Game/Blueprints/Player/Input/IA_Look.IA_Look"))
  (Pawn|Input|AddControllerYawInput (.x ActionValue))
  (Pawn|Input|AddControllerPitchInput (* (.y ActionValue) -1.0)))

(event Input|EnhancedActionEvents|EnhancedInputActionIA_Jump
  (params (ActionValue :type Boolean) (ElapsedSeconds :type Float%20%28double-precision%29) (TriggeredSeconds :type Float%20%28double-precision%29) (InputAction :type Input%20Action%20Object%20Reference :default "/Game/Blueprints/Player/Input/IA_Jump.IA_Jump"))
  (:Started
    (Character|Jump))
  (:Canceled
    (Character|StopJumping)))

(event Input|EnhancedActionEvents|EnhancedInputActionIA_Boost
  (params (ActionValue :type Boolean) (ElapsedSeconds :type Float%20%28double-precision%29) (TriggeredSeconds :type Float%20%28double-precision%29) (InputAction :type Input%20Action%20Object%20Reference :default "/Game/Blueprints/Player/Input/IA_Boost.IA_Boost"))
  (bind _charactermovement (Variables|Character|GetCharacterMovement))
  (:Started
    (Variables|Default|SetBoosting? true)
    (Variables|/Script/Engine.CharacterMovementComponent|SetMaxWalkSpeed _charactermovement (Variables|Default|GetMaxBoostSpeed))
    (bind _returnvalue (Rendering|Material|CreateDynamicMaterialInstance "/Game/Shaders/BlurVignette_Inst.BlurVignette_Inst" "None" "None" :!class /Script/Engine.KismetMaterialLibrary))
    (while (Variables|Default|GetBoosting?)
      (Physics|AddImpulse _charactermovement (* (Transformation|GetActorForwardVector) "100.000000,0.000000,0.000000") false)
      (if (not (Variables|Default|GetBoosting?))
        _))
    (Development|PrintText "Nice"))
  (:Canceled
    (Variables|Default|SetBoosting? false :!label _label)
    (Variables|/Script/Engine.CharacterMovementComponent|SetMaxWalkSpeed _charactermovement (Variables|Default|GetMaxRunSpeed))
    (Rendering|Material|SetScalarParameterValue _returnvalue "Blur Radius" 0.0 :!class /Script/Engine.MaterialInstanceDynamic)
    (Rendering|Material|SetScalarParameterValue _returnvalue "Blur" 0.0 :!class /Script/Engine.MaterialInstanceDynamic))
  (:Completed
    (goto _label)))

(event EventBeginPlay
  (bind _asplayer_controller (Utilities|Casting|CastToPlayerController (Pawn|GetController)))
  (Utilities|IsValid _asplayer_controller
    (:Is%20Valid
      (Input|AddMappingContext (PlayerController|LocalPlayerSubsystems|GetEnhancedInputLocalPlayerSubsystem _asplayer_controller) "/Game/Blueprints/Player/Input/IMC_Sonic.IMC_Sonic" 0 "(bIgnoreAllPressedKeysUntilRelease=True,bForceImmediately=False,bNotifyUserSettings=False)"))))

(event EventTick
  (params (DeltaSeconds :type Float%20%28single-precision%29))
  (bind _returnvalue (Transformation|GetVelocity))
  (bind (_x _y) (Math|Vector|BreakVector _returnvalue))
  (if (< (Variables|Default|GetBoost) 0.0)
    (Variables|Default|SetBoost 0.0))
  (if (Variables|Default|GetBoosting?)
    (Rendering|Material|SetScalarParameterValue (stale Input|EnhancedActionEvents|EnhancedInputActionIA_Boost _returnvalue) "Blur Radius" (/ (+ _x _y) 1e+03) :!class /Script/Engine.MaterialInstanceDynamic)
    (Rendering|Material|SetScalarParameterValue (stale Input|EnhancedActionEvents|EnhancedInputActionIA_Boost _returnvalue) "Blur" 0.3 :!class /Script/Engine.MaterialInstanceDynamic)
    (Rendering|AddorUpdateBlendable (Variables|Default|GetPostProcess) (stale Input|EnhancedActionEvents|EnhancedInputActionIA_Boost _returnvalue) 1.0 :!class /Script/Engine.PostProcessComponent)))

(fn ConstructionScript)

(fn GetPP
  (return 0))